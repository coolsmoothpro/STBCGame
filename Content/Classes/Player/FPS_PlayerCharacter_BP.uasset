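; First-person player character Blueprint that handles mouse look and planar movement input.
; Mouse axes drive controller yaw and inverted pitch.
; Movement axes feed AddMovementInput with the Camera's forward and right vectors, flattened to Z=0 and scaled by axis value and Speed.
; The flattened vectors are not renormalized, so forward input magnitude shrinks as the camera pitches up or down.
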(event `InputAxisKey|MouseX`
  (params (AxisValue :type "Float (single-precision)"))
  (`self.AddControllerYawInput` AxisValue))

(event `InputAxis|mouseY`
  (params (AxisValue :type "Float (single-precision)"))
  (`self.AddControllerPitchInput` (* AxisValue -1.0)))

(event `InputAxis|forward_back`
  (params (AxisValue :type "Float (single-precision)"))
  (`self.AddMovementInput` (* (`KismetMathLibrary.MakeVector` (.x (`SceneComponent.GetForwardVector` (`self.Camera`))) (.y (`SceneComponent.GetForwardVector` (`self.Camera`)))) AxisValue (`self.speed`))))

(event `InputAxis|right_left`
  (params (AxisValue :type "Float (single-precision)"))
  (`self.AddMovementInput` (* (`KismetMathLibrary.MakeVector` (.x (`SceneComponent.GetRightVector` (`self.Camera`))) (.y (`SceneComponent.GetRightVector` (`self.Camera`)))) AxisValue (`self.speed`))))

(fn `UserConstructionScript`)