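; Player controller for interactively drawing spline-based free roads with the mouse and keyboard.
; Shift+Right Mouse spawns a road through the RoadManager at the cursor hit, Space adds points, and C stops and releases it.
; Each tick updates the active road to the cursor, snapping position and direction to nearby RoadIntersectionActor connect points, otherwise using automatic direction.
; Keys 1 and 2 adjust the tangent scale of the second-to-last spline point.
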(event `self.ReceiveTick`
  (params (DeltaSeconds :type "Float (single-precision)"))
  (bind (_hitresult _returnvalue) (`self.GetHitResultUnderCursorByChannel` "TraceTypeQuery1"))
  (bind (_bblockinghit _binitialoverlap _time _distance _location _impactpoint _normal _impactnormal _physmat _hitactor) (`GameplayStatics.BreakHitResult` _hitresult))
  (`/Engine/EditorBlueprintResources/StandardMacros.IsValid` (`self.current_freeRoad`)
    (:`Is Valid`
      (if _returnvalue
        (bind _asroad_intersection_actor (cast `RoadIntersectionActor` _hitactor)
          (:`then`
            (`FreeRoadGeneratorComponent.OnUpdate` (`self.current_freeRoad`) (.location (`RoadIntersectionActor.GetConnectPointTransformNearLocation` _asroad_intersection_actor _impactpoint)) (`KismetMathLibrary.GetForwardVector` (.rotation (`RoadIntersectionActor.GetConnectPointTransformNearLocation` _asroad_intersection_actor _impactpoint))) false))
          (:`CastFailed`
            (`FreeRoadGeneratorComponent.OnUpdate` (`self.current_freeRoad`) _impactpoint (0.0 0.0 0.0) true)))))))

(event `Key|SpaceBar`
  (params (Key :type "Key Structure"))
  (bind (_hitresult _returnvalue) (`self.GetHitResultUnderCursorByChannel` "TraceTypeQuery1"))
  (bind _current_freeroad (`self.current_freeRoad`))
  (:`Pressed`
    (`/Engine/EditorBlueprintResources/StandardMacros.IsValid` (`self.current_freeRoad`)
      (:`Is Valid`
        (`/Engine/EditorBlueprintResources/StandardMacros.IsValid` _current_freeroad
          (:`Is Valid`
            (if _returnvalue
              (`FreeRoadGeneratorComponent.AddPointAtLoc` _current_freeroad (`.ImpactPoint` (`GameplayStatics.BreakHitResult` _hitresult))))))))))

(event `Key|Shift+RightMouseButton`
  (params (Key :type "Key Structure"))
  (bind _returnvalue (`self.GetRoadManager`))
  (bind (_hitresult _returnvalue_2) (`self.GetHitResultUnderCursorByChannel` "TraceTypeQuery1"))
  (:`Pressed`
    (`/Engine/EditorBlueprintResources/StandardMacros.IsValid` (`self.current_freeRoad`)
      (:`Is Not Valid`
        (`/Engine/EditorBlueprintResources/StandardMacros.IsValid` _returnvalue
          (:`Is Valid`
            (if _returnvalue_2
              (bind _returnvalue_3 (`RoadManager.AddNewFreeRoad` _returnvalue))
              (bind _output_get (set `self.current_freeRoad` _returnvalue_3))
              (`/Engine/EditorBlueprintResources/StandardMacros.IsValid` _output_get
                (:`Is Valid`
                  (`FreeRoadGeneratorComponent.OnStart` _output_get (`.ImpactPoint` (`GameplayStatics.BreakHitResult` _hitresult))))
                (:`Is Not Valid`
                  (`KismetSystemLibrary.PrintString` "spawned free Road  not invalid")))
              (else
                (`KismetSystemLibrary.PrintString` "not hIt"))))
          (:`Is Not Valid`
            (`KismetSystemLibrary.PrintString` "Road Manager not found")))))))

(event `Key|C`
  (params (Key :type "Key Structure"))
  (:`Pressed`
    (`WidgetBlueprintLibrary.SetInputMode_GameAndUIEx` self null "DoNotLock" false)
    (`FreeRoadGeneratorComponent.OnStop` (`self.current_freeRoad`) (0.0 0.0 0.0))
    (set `self.current_freeRoad` null)))

(event `Key|One`
  (params (Key :type "Key Structure"))
  (bind _current_freeroad (`self.current_freeRoad`))
  (:`Pressed`
    (`/Engine/EditorBlueprintResources/StandardMacros.IsValid` _current_freeroad
      (:`Is Valid`
        (bind _output_get (set `self.Tangent_Scaler` (`KismetMathLibrary.FClamp` (+ (`self.Tangent_Scaler`) 0.1) 0.1)))
        (`FreeRoadGeneratorComponent.UpdatePointTangentScale` (`self.current_freeRoad`) (- (`SplineComponent.GetNumberOfSplinePoints` _current_freeroad) 2) _output_get)))))

(event `Key|Two`
  (params (Key :type "Key Structure"))
  (bind _current_freeroad (`self.current_freeRoad`))
  (:`Pressed`
    (`/Engine/EditorBlueprintResources/StandardMacros.IsValid` _current_freeroad
      (:`Is Valid`
        (bind _output_get (set `self.Tangent_Scaler` (`KismetMathLibrary.FClamp` (+ (`self.Tangent_Scaler`) -0.1) 0.1)))
        (`FreeRoadGeneratorComponent.UpdatePointTangentScale` (`self.current_freeRoad`) (- (`SplineComponent.GetNumberOfSplinePoints` _current_freeroad) 2) _output_get)))))

(fn `GetRoadManager`
  (returns (ReturnValue :type "/Game/Classes/Actotrs/RoadManager_BP Object Reference"))
  (bind _returnvalue (`GameplayStatics.GetActorOfClass` "/Game/Classes/Actotrs/RoadManager_BP.RoadManager_BP_C"))
  (return _returnvalue))

(fn `UserConstructionScript`)